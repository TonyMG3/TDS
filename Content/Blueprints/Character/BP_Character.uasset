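; Top-down player character Blueprint that handles camera zoom and movement-mode input.
; Walk, sprint and right-mouse aim inputs set held-state flags, then call ChageMovementState, which is not defined in this graph.
; Mouse wheel steps the camera boom length within height limits, either instantly or through a looping timer that ignores new scrolls until finished.
; The construction script configures boom length, rotation and lag; CameraShakeEvent plays a shake at the camera.
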(event Input|ActionEvents|InputActionMovementModeChangeWalk
  (params (Key :type Key%20Structure :default "None"))
  (:Pressed
    (Variables|Default|SetWalkEnabled true)
    (Class|TopDownCharacter|ChageMovementState :!label _label))
  (:Released
    (Variables|Default|SetWalkEnabled false)
    (goto _label)))

(event Input|ActionEvents|InputActionMovementModeChangeSprint
  (params (Key :type Key%20Structure :default "None"))
  (:Pressed
    (Variables|Default|SetSprintRunEnabled true)
    (Class|TopDownCharacter|ChageMovementState :!label _label))
  (:Released
    (Variables|Default|SetSprintRunEnabled false)
    (goto _label)))

(event Input|AxisEvents|InputAxisMouseWheel
  (params (AxisValue :type Float%20%28single-precision%29))
  (if (Variables|Default|GetSlideWithSmooth)
    (CallFunction|CameraSlideSmooth AxisValue)
    (else
      (CallFunction|CameraSlide AxisValue))))

(event Input|MouseEvents|RightMouseButton
  (params (Key :type Key%20Structure :default "None"))
  (:Pressed
    (Variables|Default|SetAimEnabled true)
    (Class|TopDownCharacter|ChageMovementState :!label _label))
  (:Released
    (Variables|Default|SetAimEnabled false)
    (goto _label)))

(fn ConstructionScript
  (bind _cameraboom (Variables|Default|GetCameraBoom))
  (Variables|/Script/Engine.SpringArmComponent|SetTargetArmLength _cameraboom (Variables|Default|GetHieghtCameraMin))
  (Transformation|SetRelativeRotation _cameraboom (Variables|Default|GetRotatorCamera) false false)
  (Variables|/Script/Engine.SpringArmComponent|SetbEnableCameraLag _cameraboom (Variables|Default|Getflow))
  (Variables|/Script/Engine.SpringArmComponent|SetCameraLagSpeed _cameraboom (Variables|Default|GetCoefSmooth)))

(fn CameraShakeEvent
  (Camera|PlayWorldCameraShake "/Game/Blueprints/Game/BP_CameraShake.BP_CameraShake_C" (Transformation|GetWorldLocation (Variables|Default|GetTopDownCameraComponent)) 0.0 3e+01))

(fn CameraSlide
  (params (Value :type Float%20%28single-precision%29))
  (bind _cameraboom (Variables|Default|GetCameraBoom))
  (bind _heightcamerachangedistace (Variables|Default|GetHeightCameraChangeDistace))
  (if (!= Value 0.0)
    (if (< Value 0.0)
      (if (>= (Variables|Default|GetHeightCameraMax) (+ (Variables|/Script/Engine.SpringArmComponent|GetTargetArmLength _cameraboom) _heightcamerachangedistace))
        (Variables|/Script/Engine.SpringArmComponent|SetTargetArmLength _cameraboom (+ (Variables|/Script/Engine.SpringArmComponent|GetTargetArmLength _cameraboom) _heightcamerachangedistace)))
      (elif (<= (Variables|Default|GetHieghtCameraMin) (- (Variables|/Script/Engine.SpringArmComponent|GetTargetArmLength _cameraboom) _heightcamerachangedistace))
        (Variables|/Script/Engine.SpringArmComponent|SetTargetArmLength _cameraboom (- (Variables|/Script/Engine.SpringArmComponent|GetTargetArmLength _cameraboom) _heightcamerachangedistace))))))

(fn CameraSlideSmooth
  (params (Value :type Float%20%28single-precision%29))
  (bind _cameraboom (Variables|Default|GetCameraBoom))
  (bind _heightcamerachangedistace (Variables|Default|GetHeightCameraChangeDistace))
  (bind _targetarmlength (Variables|/Script/Engine.SpringArmComponent|GetTargetArmLength _cameraboom))
  (if (Variables|Default|GetSlideDone)
    (if (!= Value 0.0)
      (if (< Value 0.0)
        (if (>= (Variables|Default|GetHeightCameraMax) (+ _targetarmlength _heightcamerachangedistace))
          (Variables|Default|SetSlideUp true)
          (Variables|Default|SetSlideDone false :!label _label)
          (bind _returnvalue (Utilities|Time|SetTimerbyFunctionName 0 "CameraSlideSmoothTick" (Variables|Default|GetTimerStep) true))
          (Variables|Default|SetSlideTimer _returnvalue))
        (elif (<= (Variables|Default|GetHieghtCameraMin) (- _targetarmlength _heightcamerachangedistace))
          (Variables|Default|SetSlideUp false)
          (goto _label))))))

(fn CameraSlideSmoothTick
  (bind _cameraboom (Variables|Default|GetCameraBoom))
  (bind _heightchangeslidestepdistace (Variables|Default|GetHeightChangeSlideStepDistace))
  (bind _output_get (Variables|Default|SetCurrentSlideDistace (+ (Variables|Default|GetCurrentSlideDistace) _heightchangeslidestepdistace)))
  (Variables|/Script/Engine.SpringArmComponent|SetTargetArmLength _cameraboom (select (Variables|Default|GetSlideUp) (+ (Variables|/Script/Engine.SpringArmComponent|GetTargetArmLength _cameraboom) _heightchangeslidestepdistace) (- (Variables|/Script/Engine.SpringArmComponent|GetTargetArmLength _cameraboom) _heightchangeslidestepdistace)))
  (if (>= _output_get (Variables|Default|GetHeightCameraChangeDistace))
    (Variables|Default|SetCurrentSlideDistace 0.0)
    (Variables|Default|SetSlideDone true)
    (Utilities|Time|ClearandInvalidateTimerbyHandle (Variables|Default|GetSlideTimer))))